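; Health pickup that restores the player's LifeForce through its ApplyEffect event.
; Below full health it plays a click sound at the game instance's effects volume, then adds an amount that rises with game time toward 40% of full health.
; LifeForce caps at 1.0.
; Setting Speed to 999 removes the pickup when health is already full or the whole heal fits, but not on the capped branch.
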(event `self.ApplyEffect`
  (params (PlayerCharacter :type "/Game/Blueprints/BB_MyCharacter Object Reference"))
  (bind _returnvalue (`KismetSystemLibrary.GetGameTimeInSeconds`))
  (bind _lifeforce (`/Game/Blueprints/BB_MyCharacter.LifeForce` PlayerCharacter))
  (bind _returnvalue_2 (+ _lifeforce (* (/ (+ _returnvalue 0.0) (+ _returnvalue 10.0)) 0.4)))
  ;[1 1 1] Onko hp max?
  (if (>= _lifeforce 1.0)
    ;[1 1 1] Hp muutos päätös
    (set `self.Speed` 999.0 :!label _label) ; Poistaa pickupin
    (else
      ;[1 1 1] Ääniefekti
      (bind _aspeli_instanssi (cast `/Game/Blueprints/PeliInstanssi` (`GameplayStatics.GetGameInstance`)))
      (`GameplayStatics.PlaySound2D` "/Game/Sounds/ClicksEcho.ClicksEcho" (`/Game/Blueprints/PeliInstanssi.EfektienVoimakkuus` _aspeli_instanssi) 1.0 0.0 null null)
      (if (<= _returnvalue_2 1.0)
        (set `/Game/Blueprints/BB_MyCharacter.LifeForce` _returnvalue_2 PlayerCharacter)
        (goto _label)
        (else
          (set `/Game/Blueprints/BB_MyCharacter.LifeForce` 1.0 PlayerCharacter))))))

(fn `UserConstructionScript`
  (`parent.UserConstructionScript`))