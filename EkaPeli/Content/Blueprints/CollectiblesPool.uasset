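; Object pool of collectibles that scroll along +X at random heights and get recycled rather than destroyed.
; CreateCollectible spawns into ThePool up to a maximum count, randomizing speed with a bound based on elapsed game time.
; UpdateCollectibles offsets each item by its Speed per call, without delta time, and returns those past the mirrored start X with new height and speed.
; Its own events are empty, and neither function is called here.
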(fn `CreateCollectible`
  (bind _numberofcollectibles (`self.numberOfCollectibles`))
  ;[1 1 1] Onko tilaa?
  (if (< (`self.numberOfCollectibles`) (`self.maxNumberOfCollectibles`))
    ;[1 1 1] Collectible nopeus satunnaisuus.
    (bind _returnvalue (`|SpawnActorFromClass` "/Game/Blueprints/Collectible.Collectible_C" (`KismetMathLibrary.MakeTransform` (`KismetMathLibrary.MakeVector` (`self.collectibleStartX`) 0.0 (`KismetMathLibrary.RandomFloatInRange` 150.0 750.0))) "Undefined" "OverrideRootScale" null null))
    (bind _speed (`/Game/Blueprints/Collectible.Speed` _returnvalue))
    (set `/Game/Blueprints/Collectible.Speed` (`KismetMathLibrary.RandomFloatInRange` (/ _speed (/ (`KismetSystemLibrary.GetGameTimeInSeconds`) 10.0)) _speed) _returnvalue)
    ;[1 1 1] Luotu objekti altaaseen
    (`KismetArrayLibrary.Array_Insert` (`self.thePool`) _returnvalue _numberofcollectibles)
    (`/Engine/EditorBlueprintResources/StandardMacros.IncrementInt` _numberofcollectibles)))

(fn `UpdateCollectibles`
  (locals (arrayElement :type "/Game/Blueprints/Collectible Object Reference") (arrayIndex :type Integer))
  ;[1 1 1] Päivitä kaikki poolin osat
  (for (_array_element _array_index) (`self.thePool`)
    ;[1 1 1] Teleport tarkistus
    (set `local.arrayElement` _array_element)
    (set `local.arrayIndex` _array_index)
    (bind _rootcomponent (`Actor.RootComponent` _array_element))
    (if (> (.x (`SceneComponent.K2_GetComponentLocation` _rootcomponent)) (- 0.0 (`self.collectibleStartX`)))
      ;[1 1 1] Teleporttaa collectible
      (`SceneComponent.K2_SetWorldLocation` (`Actor.RootComponent` (`local.arrayElement`)) (`KismetMathLibrary.MakeVector` (`self.collectibleStartX`) 0.0 (`KismetMathLibrary.RandomFloatInRange` 150.0 750.0)) false false)
      (set `/Game/Blueprints/Collectible.Speed` (`KismetMathLibrary.RandomFloatInRange` 10.0 15.0) (`local.arrayElement`))
      (else
        ;[1 1 1] Liikuta collectible
        (`SceneComponent.K2_AddWorldOffset` _rootcomponent (`KismetMathLibrary.MakeVector` (`/Game/Blueprints/Collectible.Speed` _array_element)) false false)))))

(fn `UserConstructionScript`)