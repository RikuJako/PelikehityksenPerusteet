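; NopeusVahennys is a speed-penalty item that temporarily changes the player's speed bonus when its effect is applied.
; ApplyEffect sets the item's Speed very high to remove it, then, unless already active, plays a whoosh at the game instance's effects volume.
; NopeusMuutos adds Penalty to the player's NopeusBonus, then subtracts it after a five-second delay, with the Aktiivinen flag blocking re-triggering meanwhile.
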(event `self.ApplyEffect`
  (params (PlayerCharacter :type "/Game/Blueprints/BB_MyCharacter Object Reference"))
  (bind _pelaaja (`self.Pelaaja`))
  (bind _penalty (`self.Penalty`))
  (set `self.Pelaaja` PlayerCharacter)
  (set `self.Speed` 999.0) ; Poistetaan esine
  (if (not (`self.Aktiivinen`))
    ;[1 1 1] Ääniefekti
    (bind _aspeli_instanssi (cast `/Game/Blueprints/PeliInstanssi` (`GameplayStatics.GetGameInstance`)))
    (`GameplayStatics.PlaySound2D` "/Game/Sounds/Woosh.Woosh" (`/Game/Blueprints/PeliInstanssi.EfektienVoimakkuus` _aspeli_instanssi) 1.0 0.0 null null)
    (set `self.Aktiivinen` true) ; Kielletään uusi bonus
    (`self.NopeusMuutos` _pelaaja _penalty) ; Annetaan penalty
    (`KismetSystemLibrary.Delay` 5.0) ; Bonuksen kesto
    (`self.NopeusMuutos` _pelaaja (- 0.0 _penalty)) ; Poistetaan penalty
    (set `self.Aktiivinen` false) ; Sallitaan uusi bonus
  ))

(fn `NopeusMuutos`
  (params (Kohde :type "/Game/Blueprints/BB_MyCharacter Object Reference") (Muutos :type "Float (double-precision)"))
  (bind _output_get (set `/Game/Blueprints/BB_MyCharacter.NopeusBonus` (+ (`/Game/Blueprints/BB_MyCharacter.NopeusBonus` Kohde) Muutos) Kohde)))

(fn `UserConstructionScript`
  (`parent.UserConstructionScript`))