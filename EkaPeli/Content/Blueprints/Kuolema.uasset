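; Kuolema ("death") is a hazard actor that kills the player character when its effect is applied.
; Tick spins its laser sprite around the pitch axis by a fixed step each frame, independent of delta time.
; ApplyEffect calls KillMe on the player; this Blueprint's own overlap event is disabled, so the trigger lives outside this graph.
; Unconnected legacy nodes for a crouch flipbook and direct health changes never run.
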(event `self.ReceiveTick`
  (params (DeltaSeconds :type "Float (single-precision)"))
  ;[1 1 1] Pyöritetään spriteä
  (bind _returnvalue (+ (stale _output_get) 5))
  (bind _output_get (set `self.Rotaatio` _returnvalue))
  (`SceneComponent.K2_SetWorldRotation` (`self.laser-98735_960_720_Sprite`) (`KismetMathLibrary.MakeRotator` 0.0 (`KismetMathLibrary.Conv_IntToDouble` _returnvalue)) false false))

(event `self.ApplyEffect`
  (params (PlayerCharacter :type "/Game/Blueprints/BB_MyCharacter Object Reference"))
  ;[1 1 1] Tapetaan pelaaja
  (`/Game/Blueprints/BB_MyCharacter.KillMe` PlayerCharacter))

(fn `UserConstructionScript`
  (`parent.UserConstructionScript`))