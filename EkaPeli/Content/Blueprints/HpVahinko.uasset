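; HpVahinko ("HP damage") is a harmful item that lowers the player's LifeForce when its ApplyEffect event fires.
; Damage scales with elapsed game time as a difficulty curve approaching 0.3, and is negative during the first four seconds.
; It calls KillMe when LifeForce is no longer positive.
; Either way, it sets its Speed very high to remove itself and plays one of two random pain sounds.
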(event `self.ApplyEffect`
  (params (PlayerCharacter :type "/Game/Blueprints/BB_MyCharacter Object Reference"))
  (bind _returnvalue (`KismetSystemLibrary.GetGameTimeInSeconds`))
  (bind _output_get (set `/Game/Blueprints/BB_MyCharacter.LifeForce` (- (`/Game/Blueprints/BB_MyCharacter.LifeForce` PlayerCharacter) (* (/ (+ _returnvalue -4.0) (+ _returnvalue 5.0)) 0.3)) PlayerCharacter)) ; Vähennetään hp:ta
  (if (not (> _output_get 0.0))
    (`/Game/Blueprints/BB_MyCharacter.KillMe` PlayerCharacter))
  (set `self.Speed` 999.0) ; Poistetaan esine
  (if (`KismetMathLibrary.RandomBool`)
    (`GameplayStatics.PlaySound2D` "/Game/Sounds/SpeechAugh.SpeechAugh" 1.0 1.0 0.0 null null)
    (else
      (`GameplayStatics.PlaySound2D` "/Game/Sounds/SpeechAugh2.SpeechAugh2" 1.0 1.0 0.0 null null))))

(fn `UserConstructionScript`
  (`parent.UserConstructionScript`))