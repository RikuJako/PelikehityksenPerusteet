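; AikaBonus is a time bonus pickup that adds to the player's survival-time bonus.
; It overrides ApplyEffect to add its AikaBonus value to the PlayerCharacter's HengissaAikaBonus.
; It then removes itself by setting Speed very high rather than destroying the actor.
; It finishes with a ticking-clock sound at the effects volume stored in the PeliInstanssi game instance.
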(event `self.ApplyEffect`
  (params (PlayerCharacter :type "/Game/Blueprints/BB_MyCharacter Object Reference"))
  (set `/Game/Blueprints/BB_MyCharacter.HengissaAikaBonus` (+ (`/Game/Blueprints/BB_MyCharacter.HengissaAikaBonus` PlayerCharacter) (`self.AikaBonus`)) PlayerCharacter) ; Tallennetaan ajan muutos
  (set `self.Speed` 999.0) ; Poistetaan esine
  ;[1 1 1] Ääniefekti
  (bind _aspeli_instanssi (cast `/Game/Blueprints/PeliInstanssi` (`GameplayStatics.GetGameInstance`)))
  (`GameplayStatics.PlaySound2D` "/Game/Sounds/ClockTickingSlow.ClockTickingSlow" (`/Game/Blueprints/PeliInstanssi.EfektienVoimakkuus` _aspeli_instanssi) 5.0 8.0 null null))

(fn `UserConstructionScript`
  (`parent.UserConstructionScript`))